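; BP_Cannon is a turret actor that tracks the first player's pawn and periodically spawns an actor aimed at it.
; Tick rotates the Arrow component with a look-at rotation from the cannon's location to player 0's pawn.
; A looping timer started on BeginPlay spawns the actor at the cannon's location using the Arrow's world rotation.
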(event Custom|OnTimerElapsed
  (Game|SpawnActorfromClass "/Game/HordeMp/BP_HMP_Projectile.BP_HMP_Projectile_C" (Math|Transform|MakeTransform (Transformation|GetActorLocation) (Transformation|GetWorldRotation (Variables|Default|GetArrow))) "Undefined" "MultiplyWithRoot" 0 0))

(event EventBeginPlay
  (Utilities|Time|SetTimerbyEvent (delegate Custom|OnTimerElapsed) 2.0 true))

(event Collision|EventActorBeginOverlap
  (params (OtherActor :type Actor%20Object%20Reference)))

(event EventTick
  (params (DeltaSeconds :type Float%20%28single-precision%29))
  (Transformation|SetWorldRotation (Variables|Default|GetArrow) (Math|Rotator|FindLookatRotation (Transformation|GetActorLocation) (Transformation|GetActorLocation (Game|Player|GetPlayerPawn 0))) false false))

(fn ConstructionScript)