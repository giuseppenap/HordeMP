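; Player controller for the HordeMp game mode that sets up the local player's HUD and handles two shortcut keys.
; On BeginPlay, only for the local controller, it caches BP_HMP_MainHUD, pushes the HUD widget through the HUD's DebugMenu and sets game-only input.
; DebugKey2 pushes the pause menu onto that same DebugMenu.
; The L key writes a save game through HMP_GameModeBase and prints a confirmation.
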(event EventBeginPlay
  (if (Pawn|IsLocalController)
    (bind _asbp_hmp_main_hud (Utilities|Casting|CastToBP_HMP_MainHUD (HUD|GetHUD)))
    (Variables|Default|SetHUD_Ref _asbp_hmp_main_hud)
    (bind _widget (Default|DebugMenu (Variables|Default|GetHUD_Ref)))
    (Default|PushWidget _widget "/Game/HordeMp/UI/StackableWidgets/WBP_HUD.WBP_HUD_C")
    (Input|SetInputModeGameOnly self false)))

(event Input|KeyboardEvents|DebugKey2
  (params (Key :type Key%20Structure :default "None") (ActionValue :type Input%20Action%20Value%20Structure))
  (:Pressed
    (bind _widget (Default|DebugMenu (Variables|Default|GetHUD_Ref)))
    (Default|PushWidget _widget "/Game/HordeMp/UI/Menu/WBP_PauseMenu.WBP_PauseMenu_C")))

(event Input|KeyboardEvents|L
  (params (Key :type Key%20Structure :default "None"))
  (:Pressed
    (bind _ashmp_game_mode_base (Utilities|Casting|CastToHMP_GameModeBase (Game|GetGameMode)))
    (Class|HMPGameModeBase|WriteSaveGame _ashmp_game_mode_base)
    (Development|PrintString "World has been saved" true true "(R=0.000000,G=0.660000,B=1.000000,A=1.000000)" 5.0)))

(fn ConstructionScript)