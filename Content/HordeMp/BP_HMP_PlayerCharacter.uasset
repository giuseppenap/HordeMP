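; BP_HMP_PlayerCharacter is the player character Blueprint for the HordeMp game mode or module.
; On BeginPlay it creates a minion health widget attached to itself and adds it to the viewport.
; The Parry input starts the Parry action by name on its action component, and a debug key applies damage through the attribute component.
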(event EventBeginPlay
  (bind _returnvalue (UserInterface|CreateWidget "/Game/HordeMp/UI/WBP_MinionHealth.WBP_MinionHealth_C" 0 self))
  (UserInterface|Viewport|AddtoViewport _returnvalue 0))

(event Input|ActionEvents|InputActionParry
  (params (Key :type Key%20Structure))
  (:Pressed
    (Class|HMPActionComponent|StartActionbyName (Variables|Default|GetActionComp) self "Parry")))

(event Input|KeyboardEvents|DebugKey4
  (params (Key :type Key%20Structure) (ActionValue :type Input%20Action%20Value%20Structure))
  (:Pressed
    (Class|HMPAttributeComponent|ApplyHealthChange (Variables|Default|GetAttributeComp) self -3e+01)))

(fn ConstructionScript)