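; BP_HMP_Cannon is a turret that tracks the first player and fires projectiles at them automatically.
; Tick rotates its Arrow component to face player pawn 0.
; A looping two-second timer, started at BeginPlay, spawns a BP_HMP_FireProjectile at the actor's location with the Arrow's rotation.
; It then sets InitialSpeed on the projectile's movement component, after the spawn has completed.
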(event Custom|OnTimerElapsed
  (bind _returnvalue (Game|SpawnActorfromClass "/Game/HordeMp/Projectiles/BP_HMP_FireProjectile.BP_HMP_FireProjectile_C" (Math|Transform|MakeTransform (Transformation|GetActorLocation) (Transformation|GetWorldRotation (Variables|Default|GetArrow))) "Undefined" "MultiplyWithRoot" 0 0))
  (Variables|/Script/Engine.ProjectileMovementComponent|SetInitialSpeed (Actor|GetComponentbyClass _returnvalue "/Script/Engine.ProjectileMovementComponent") 5e+03))

(event EventBeginPlay
  (Utilities|Time|SetTimerbyEvent (delegate Custom|OnTimerElapsed) 2.0 true))

(event Collision|EventActorBeginOverlap
  (params (OtherActor :type Actor%20Object%20Reference)))

(event EventTick
  (params (DeltaSeconds :type Float%20%28single-precision%29))
  (Transformation|SetWorldRotation (Variables|Default|GetArrow) (Math|Rotator|FindLookatRotation (Transformation|GetActorLocation) (Transformation|GetActorLocation (Game|Player|GetPlayerPawn 0))) false false))

(fn ConstructionScript)