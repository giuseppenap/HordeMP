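; BP_DashFogCard2 is a placeable fog card actor for the Cemetery Crypt environment that renders wind-driven cloud fog.
; Its construction script creates a dynamic instance of the cloud master material on the DashFogCard2 component.
; It then pushes the actor's variables for tint, density, brightness, contrast, wind and edge and camera fading into that material.
; The event graph holds only disabled stub events, so the actor runs no gameplay logic.
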(event EventBeginPlay)

(event Collision|EventActorBeginOverlap
  (params (OtherActor :type Actor%20Object%20Reference)))

(event EventTick
  (params (DeltaSeconds :type Float%20%28single-precision%29)))

(fn ConstructionScript
  (bind _returnvalue (Rendering|Material|CreateDynamicMaterialInstance (Variables|Default|GetDashFogCard2) 0 (Variables|DashProperties|GetCloud_Master_Material) "None" :!class /Script/Engine.PrimitiveComponent))
  (bind _output_get (Variables|DashProperties|SetCloud_Material_Instance _returnvalue))
  (Rendering|Material|SetVectorParameterValue _output_get "Base_Color_Tint" (Variables|DashProperties|GetBase%20Color%20Tint) :!class /Script/Engine.MaterialInstanceDynamic)
  (Rendering|Material|SetScalarParameterValue _output_get "Distance_fade" (Variables|DashProperties|GetEdge%20Fading%20Distance) :!class /Script/Engine.MaterialInstanceDynamic)
  (Rendering|Material|SetScalarParameterValue _output_get "Fog_Density" (Variables|DashProperties|GetCloud%20Density) :!class /Script/Engine.MaterialInstanceDynamic)
  (Rendering|Material|SetScalarParameterValue _output_get "Camera_Fading_Distance" (Variables|DashProperties|GetCamera%20Fading%20Distance) :!class /Script/Engine.MaterialInstanceDynamic)
  (Rendering|Material|SetScalarParameterValue _output_get "Emissive_Intensity" (Variables|DashProperties|GetCloud%20Brightness) :!class /Script/Engine.MaterialInstanceDynamic)
  (Rendering|Material|SetScalarParameterValue _output_get "Wind_Velocity" (Variables|DashProperties|GetWind%20Speed) :!class /Script/Engine.MaterialInstanceDynamic)
  (Rendering|Material|SetScalarParameterValue _output_get "Cloud_Wind_Tilling" (Variables|DashProperties|GetCloud%20Wind%20Tilling) :!class /Script/Engine.MaterialInstanceDynamic)
  (Rendering|Material|SetScalarParameterValue _output_get "Contrast_Intensity" (Variables|DashProperties|GetCloud%20Contrast) :!class /Script/Engine.MaterialInstanceDynamic)
  (Rendering|Material|SetScalarParameterValue _output_get "Wind_Direction" (Variables|DashProperties|GetWind%20Direction) :!class /Script/Engine.MaterialInstanceDynamic))